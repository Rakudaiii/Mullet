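; BP_Enemy is an AI enemy with health and fight-system components and debug-style widgets showing health, shooting readiness and walk speed.
; On BeginPlay it starts three fast looping timers, apparently for the widget updates, and sets EnumKey on the BP_AIController blackboard.
; The update functions read the components and character movement to set the health bar, can-shoot icon and speed text.
; Tick and the death handler are empty.
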(event OnDead(HealthComponent))

(event EventBeginPlay
  (Utilities|Time|SetTimerbyEvent (EventDispatchers|CreateEvent :!event UpdateHealthBar) 0.1 true)
  (Utilities|Time|SetTimerbyEvent (EventDispatchers|CreateEvent :!event UpdateCanShoot) 0.1 true)
  (Utilities|Time|SetTimerbyEvent (EventDispatchers|CreateEvent :!event UpdateWalkSpeed) 0.1 true)
  (bind _asbp_aicontroller (Utilities|Casting|CastToBP_AIController (Pawn|GetController)))
  (AI|Components|Blackboard|SetValueasEnum (Variables|/Script/AIModule.AIController|GetBlackboard _asbp_aicontroller) (Utilities|Name|MakeLiteralName "EnumKey") 1))

(event EventTick
  (params (DeltaSeconds :type Float%20%28single-precision%29)))

(fn ConstructionScript)

(fn UpdateHealthBar
  (bind _aswbp_show_enemy_health (Utilities|Casting|CastToWBP_ShowEnemyHealth (UserInterface|GetWidget (Variables|Default|GetWBP_Health))))
  (bind _returnvalue (Class|MDJHealthComponent|GetCurrentHealth (Variables|Default|GetHealthComponent)))
  (bind _returnvalue_2 (Class|MDJHealthComponent|GetMaxHealth (Variables|Default|GetHealthComponent)))
  (Progress|SetPercent (Variables|/Game/MulletMadJack/UI/DebugUI/WBP_ShowEnemyHealth.WBP_ShowEnemyHealth_C|GetHealthBar _aswbp_show_enemy_health) (Math|Float|MapRangeClamped _returnvalue 0.0 _returnvalue_2 0.0 1.0)))

(fn UpdateCanShoot
  (bind _returnvalue (Class|MDJFightSystemComponent|GetbCanShoot (Variables|Default|GetFightSystemComponent)))
  (bind _aswbp_show_can_shooting (Utilities|Casting|CastToWBP_ShowCanShooting (UserInterface|GetWidget (Variables|Default|GetWBP_Shoot))))
  (if _returnvalue
    (Appearance|SetBrushfromTexture (Variables|/Game/MulletMadJack/UI/DebugUI/WBP_ShowCanShooting.WBP_ShowCanShooting_C|GetImage_82 _aswbp_show_can_shooting) "/Game/MulletMadJack/UI/DebugUI/Image/CanShoot.CanShoot" false)
    (else
      (Appearance|SetBrushfromTexture (Variables|/Game/MulletMadJack/UI/DebugUI/WBP_ShowCanShooting.WBP_ShowCanShooting_C|GetImage_82 _aswbp_show_can_shooting) "/Game/MulletMadJack/UI/DebugUI/Image/CantShoot.CantShoot" false))))

(fn UpdateWalkSpeed
  (bind _aswbp_show_walk_speed (Utilities|Casting|CastToWBP_ShowWalkSpeed (UserInterface|GetWidget (Variables|Default|GetWBP_WalkSpeed))))
  (Rendering|Components|TextRender|SetText (Variables|/Game/MulletMadJack/UI/DebugUI/WBP_ShowWalkSpeed.WBP_ShowWalkSpeed_C|GetText_WalkSpeed _aswbp_show_walk_speed) (Utilities|Text|ToText(Integer) (Math|Float|Truncate (Variables|/Script/Engine.CharacterMovementComponent|GetMaxWalkSpeed (Variables|Character|GetCharacterMovement))))))